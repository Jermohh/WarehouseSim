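; BP_OfficeDoor is a double-door Blueprint that swings its two leaves open and closed through a toggling OpenDoor event.
; The DoorOpen timeline lerps the left and right pivots to opposite 90-degree yaw rotations, with sweep enabled.
; Each call flips IsDoorOpen: a true value plays the timeline forward to swing the leaves out, and a false value reverses it from the end.
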(event Custom|OpenDoor
  (if (Variables|Default|GetIsDoorOpen)
    (Variables|Default|SetIsDoorOpen false)
    (bind _dooropen (Timeline|DoorOpen Play)
      (:Update
        (Transformation|SetRelativeRotation (Variables|Default|GetLeftDoorPivot) (Math|Rotator|Lerp(Rotator) "0, 0, 0" "0.000000,-90.000000,0.000000" _dooropen) true false)
        (Transformation|SetRelativeRotation (Variables|Default|GetRightDoorPivot) (Math|Rotator|Lerp(Rotator) "0, 0, 0" "0.000000,90.000000,0.000000" _dooropen) true false)))
    (else
      (Variables|Default|SetIsDoorOpen true)
      (Timeline|DoorOpen ReverseFromEnd))))

(fn ConstructionScript)