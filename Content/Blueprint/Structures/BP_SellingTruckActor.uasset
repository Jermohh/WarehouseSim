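; BP_SellingTruckActor is a selling truck actor that drives away and returns to where it started.
; BeginPlay stores the starting location, and DriveTruckAway plays the TruckSelling timeline to lerp the truck along world X from its current location with a swept move.
; ReturnTruck resets the lerp origin to the stored start and reverses the same timeline from its end.
; Debug prints trace the locations and the return call.
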(event EventBeginPlay
  (bind _output_get (Variables|Default|SetInitialTruckStartingLocation (Transformation|GetActorLocation)))
  (Development|PrintString (Utilities|String|ToString(Vector) _output_get)))

(event EventDriveTruckAway
  (bind _output_get (Variables|Default|SetCurrentTruckLocation (Transformation|GetActorLocation)))
  (Development|PrintString (Utilities|String|ToString(Vector) _output_get))
  (bind _newtrack_0 (Timeline|TruckSelling Play)
    (:Update
      (Transformation|SetActorLocation (Math|Vector|Lerp(Vector) (Variables|Default|GetCurrentTruckLocation) (+ (Variables|Default|GetCurrentTruckLocation) (Math|Vector|MakeVector 5e+03 0.0 0.0)) _newtrack_0) true false))))

(event EventReturnTruck
  (Variables|Default|SetCurrentTruckLocation (Variables|Default|GetInitialTruckStartingLocation))
  (Development|PrintString "ReturnTruckIscalled")
  (bind _newtrack_0 (Timeline|TruckSelling ReverseFromEnd)
    (:Update
      (Transformation|SetActorLocation (Math|Vector|Lerp(Vector) (Variables|Default|GetCurrentTruckLocation) (+ (Variables|Default|GetCurrentTruckLocation) (Math|Vector|MakeVector 5e+03 0.0 0.0)) _newtrack_0) true false))))

(fn ConstructionScript)