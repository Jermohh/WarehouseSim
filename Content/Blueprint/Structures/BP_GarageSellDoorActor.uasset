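; BP_GarageSellDoorActor is a door actor, named for a garage sell area, that slides vertically between open and closed positions.
; It records its open location on BeginPlay, and one shared timeline drives a swept location lerp over a configurable drop distance.
; Closing plays downward from the current location, while opening reverses from the timeline's end back to the recorded location, with debug prints for both.
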(event EventBeginPlay
  (Variables|Default|SetInitalDoorOpenLocation (Transformation|GetActorLocation)))

(event EventPlayCloseDoorTimeline
  (Variables|Default|SetDoorStartLocation (Transformation|GetActorLocation))
  (Development|PrintString "Close Door")
  (bind _doorprogress (Timeline|DoorTimeline Play)
    (:Update
      (Transformation|SetActorLocation (Math|Vector|Lerp(Vector) (Variables|Default|GetDoorStartLocation) (- (Variables|Default|GetDoorStartLocation) (Math|Vector|MakeVector 0.0 0.0 (Variables|Default|GetDoorMoveDistance))) _doorprogress) true false))))

(event EventPlayOpenDoorTimeline
  (Variables|Default|SetDoorStartLocation (Variables|Default|GetInitalDoorOpenLocation))
  (Development|PrintString "Open Door")
  (bind _doorprogress (Timeline|DoorTimeline ReverseFromEnd)
    (:Update
      (Transformation|SetActorLocation (Math|Vector|Lerp(Vector) (Variables|Default|GetDoorStartLocation) (- (Variables|Default|GetDoorStartLocation) (Math|Vector|MakeVector 0.0 0.0 (Variables|Default|GetDoorMoveDistance))) _doorprogress) true false))))

(fn ConstructionScript)