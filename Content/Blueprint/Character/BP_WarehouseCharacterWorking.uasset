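; Warehouse player character that toggles an on-screen helper widget and opens office doors on input.
; BeginPlay creates WBP_Helper, and a FlipFlop on the Helper input adds or removes it from the viewport.
; Actor overlaps cache the BP_OfficeDoor and set an in-range flag, which lets the OpenOfficeDoor input call ServerOpenDoor to open that door.
; Save and load debug prints are left disconnected.
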(event Custom|ServerOpenDoor
  (Utilities|IsValid (Variables|Default|GetAs%20BP%20Office%20Door)
    (:Is%20Valid
      (Default|OpenDoor (Variables|Default|GetAs%20BP%20Office%20Door)))))

(event EventBeginPlay
  (bind _returnvalue (UserInterface|CreateWidget "/Game/Blueprint/HUD/WBP_Helper.WBP_Helper_C"))
  (Variables|Default|SetHelper _returnvalue))

(event Collision|EventActorBeginOverlap
  (params (OtherActor :type Actor%20Object%20Reference))
  (bind _asbp_office_door (Utilities|Casting|CastToBP_OfficeDoor OtherActor))
  (Variables|Default|SetAs%20BP%20Office%20Door _asbp_office_door)
  (Variables|Default|SetIsOverlappedWithDoor true))

(event Collision|EventActorEndOverlap
  (params (OtherActor :type Actor%20Object%20Reference))
  (Utilities|Casting|CastToBP_OfficeDoor OtherActor)
  (Variables|Default|SetIsOverlappedWithDoor false))

(event Input|ActionEvents|InputActionOpenOfficeDoor
  (params (Key :type Key%20Structure :default "None"))
  (:Pressed
    (if (Variables|Default|GetIsOverlappedWithDoor)
      (CallFunction|ServerOpenDoor))))

(event Input|ActionEvents|InputActionHelper
  (params (Key :type Key%20Structure :default "None"))
  (bind _helper (Variables|Default|GetHelper))
  (:Pressed
    (Utilities|FlowControl|FlipFlop
      (:A
        (UserInterface|Viewport|AddtoViewport _helper 0))
      (:B
        (Widget|RemovefromParent _helper)))))

(event Input|ActionEvents|InputActionSaveGame
  (params (Key :type Key%20Structure :default "None")))

(event Input|ActionEvents|InputActionLoadGame
  (params (Key :type Key%20Structure :default "None")))

(fn ConstructionScript)